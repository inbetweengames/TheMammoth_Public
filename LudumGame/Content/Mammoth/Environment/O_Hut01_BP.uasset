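; Destructible hut obstacle that the player mammoth smashes by charging into it.
; On a hit, it casts the other actor to the player mammoth and reacts only while that mammoth is charging.
; It then disables the capsule's collision, spawns a hit particle effect, swaps the intact sprite for the destroyed one and calls the HutDestroyed event dispatcher.
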(event EventBeginPlay)

(event EventTick
  (params (DeltaSeconds :type Float%20%28single-precision%29)))

(event Collision|EventHit
  (params (MyComp :type Primitive%20Component%20Object%20Reference) (Other :type Actor%20Object%20Reference) (OtherComp :type Primitive%20Component%20Object%20Reference) (bSelfMoved :type Boolean) (HitLocation :type Vector) (HitNormal :type Vector :default "0, 0, 0") (NormalImpulse :type Vector :default "0, 0, 0") (Hit :type Hit%20Result%20Structure%20%28by%20ref%29))
  (bind _obstaclesprite (Variables|Default|GetObstacleSprite))
  (bind _asc_player_mammoth_bp (Utilities|Casting|CastToC_PlayerMammoth_BP Other))
  (bind _returnvalue (Class|TPTopDownCharacter|IsCharging _asc_player_mammoth_bp))
  (if _returnvalue
    (Collision|SetCollisionEnabled (Variables|Default|GetCapsule) "NoCollision")
    (Effects|SpawnEmitteratLocation "/Game/Mammoth/Particles/HutHitFeedback.HutHitFeedback" (Transformation|GetWorldLocation _obstaclesprite))
    (Rendering|SetVisibility _obstaclesprite false false)
    (Rendering|SetVisibility (Variables|Default|GetObstacleSpriteDestroyed) true false)
    (Default|CallHutDestroyed)))

(fn ConstructionScript
  (|CallParentFunction))