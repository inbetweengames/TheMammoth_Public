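; Player mammoth Blueprint that handles the narrative voice-over, intro and ability feedback for the player's character.
; VO events about children and hunters map to timed, sometimes chained subtitles forwarded to MammothPlayerController_BP, all sharing one placeholder-like sound cue.
; Game start plays an assigned Matinee with opening lines, or without one sets the controller in-game and enables charge and trumpet UI.
; Charge and trumpet events spawn attached sounds, with dust for charging.
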(event Custom|SetSubtitle
  (params (Subtitle :type Text) (ForDuration :type Float%20%28single-precision%29) (VO :type Sound%20Cue%20Object%20Reference))
  (bind _asmammoth_player_controller_bp (Utilities|Casting|CastToMammothPlayerController_BP (Pawn|GetController)))
  (Default|SetSubtitle _asmammoth_player_controller_bp Subtitle ForDuration VO))

(event Custom|SetMatinee
  (params (Matinee :type Matinee%20Actor%20Object%20Reference))
  (Variables|Default|SetMatinee Matinee))

(event EventOnTrumpet
  (Audio|SpawnSoundAttached "/Game/Mammoth/Audio/Trumpet.Trumpet" (Variables|Default|GetCapsuleComponent) "None" "0, 0, 0" "0, 0, 0" "KeepRelativeOffset" true 1.0))

(event EventOnCharge
  (bind _capsulecomponent (Variables|Default|GetCapsuleComponent))
  (Audio|SpawnSoundAttached "/Game/Mammoth/Audio/Charge.Charge" _capsulecomponent "None" "0, 0, 0" "0, 0, 0" "KeepRelativeOffset" true)
  (Effects|SpawnEmitterAttached "/Game/Mammoth/Particles/ChargingDust.ChargingDust" _capsulecomponent "None" "0.000000,0.000000,0.000000"))

(event EventOnPlayVOEvent
  (params (event :type ESystematicVOEvent%20Enum :default "ChildrenAbandoned"))
  (switch Utilities|FlowControl|Switch|SwitchonESystematicVOEvent event
    (:ChildrenAbandoned
      (CallFunction|SetSubtitle "VO abandon" 5.0 "/Engine/EditorSounds/Notifications/CompileStart_Cue.CompileStart_Cue"))
    (:ChildrenAllDead
      (CallFunction|SetSubtitle "VO lost children" 3.0 "/Engine/EditorSounds/Notifications/CompileStart_Cue.CompileStart_Cue")
      (Utilities|FlowControl|Delay 4.0)
      (CallFunction|SetSubtitle "VO no mother" 3.0 "/Engine/EditorSounds/Notifications/CompileStart_Cue.CompileStart_Cue"))
    (:ChildSmallDead
      (CallFunction|SetSubtitle "VO lost small" 5.0 "/Engine/EditorSounds/Notifications/CompileStart_Cue.CompileStart_Cue"))
    (:ChildMiddleDead
      (CallFunction|SetSubtitle "VO lost middle" 5.0 "/Engine/EditorSounds/Notifications/CompileStart_Cue.CompileStart_Cue"))
    (:ChildBigDead
      (CallFunction|SetSubtitle "VO list eldest" 5.0 "/Engine/EditorSounds/Notifications/CompileStart_Cue.CompileStart_Cue"))
    (:ChildFollowing
      (Utilities|FlowControl|Delay 1.5)
      (CallFunction|SetSubtitle "VO found child" 2.0 "/Engine/EditorSounds/Notifications/CompileStart_Cue.CompileStart_Cue")
      (Utilities|FlowControl|Delay 4.0)
      (CallFunction|SetSubtitle "VO go east" 3.0 "/Engine/EditorSounds/Notifications/CompileStart_Cue.CompileStart_Cue"))
    (:ChildrenFollowing
      (Utilities|FlowControl|Delay 2.5)
      (CallFunction|SetSubtitle "VO child follow" 5.0 "/Engine/EditorSounds/Notifications/CompileStart_Cue.CompileStart_Cue"))
    (:ChildTakesDamage
      (CallFunction|SetSubtitle "VO hunt weak" 3.0 "/Engine/EditorSounds/Notifications/CompileStart_Cue.CompileStart_Cue")
      (Utilities|FlowControl|Delay 3.0)
      (CallFunction|SetSubtitle "VO hunt weak 2" 3.0 "/Engine/EditorSounds/Notifications/CompileStart_Cue.CompileStart_Cue"))
    (:ChildrenTakeDamage
      (CallFunction|SetSubtitle "VO child hurt" 5.0 "/Engine/EditorSounds/Notifications/CompileStart_Cue.CompileStart_Cue"))
    (:HuntersWithinRadius
      (CallFunction|SetSubtitle "VO hunters waiting" 5.0 "/Engine/EditorSounds/Notifications/CompileStart_Cue.CompileStart_Cue"))
    (:PlayerDominating
      (CallFunction|SetSubtitle "VO hunters hunted" 5.0 "/Engine/EditorSounds/Notifications/CompileStart_Cue.CompileStart_Cue"))
    (:HuntersAppear
      (CallFunction|SetSubtitle "VO more hunters" 5.0 "/Engine/EditorSounds/Notifications/CompileStart_Cue.CompileStart_Cue"))
    (:PlayerInvincible
      (CallFunction|SetSubtitle "VO no damage" 5.0 "/Engine/EditorSounds/Notifications/CompileStart_Cue.CompileStart_Cue"))))

(event EventOnGameStarted
  (bind _matinee (Variables|Default|GetMatinee))
  (Utilities|IsValid _matinee
    (:Is%20Valid
      (Audio|Components|Audio|Play _matinee)
      (Rendering|SetVisibility (Variables|Default|GetFakeFringe) false false)
      (Audio|PlaySound2D 0)
      (CallFunction|SetSubtitle "VO open 1" 2.2 "/Engine/EditorSounds/Notifications/CompileStart_Cue.CompileStart_Cue")
      (Utilities|FlowControl|Delay 3.0)
      (CallFunction|SetSubtitle "VO open 2" 2.2 "/Engine/EditorSounds/Notifications/CompileStart_Cue.CompileStart_Cue")
      (Utilities|FlowControl|Delay 3.0)
      (CallFunction|SetSubtitle "VO open 3" 2.0 "/Engine/EditorSounds/Notifications/CompileStart_Cue.CompileStart_Cue")
      (Utilities|FlowControl|Delay 3.0)
      (CallFunction|SetSubtitle "VO open 4" 2.0 "/Engine/EditorSounds/Notifications/CompileStart_Cue.CompileStart_Cue"))
    (:Is%20Not%20Valid
      (bind _astp_top_down_player_controller (Utilities|Casting|CastToTP_TopDownPlayerController (Pawn|GetController)))
      (Class|TPTopDownPlayerController|SetGameFlowState _astp_top_down_player_controller "InGame")
      (Variables|/Script/LudumGame.TP_TopDownPlayerController|Setm_isChargeUIOn _astp_top_down_player_controller true)
      (Variables|/Script/LudumGame.TP_TopDownPlayerController|Setm_isTrumpetUIOn _astp_top_down_player_controller true))))

(fn ConstructionScript)

(fn GetSpearBox
  (return (Variables|Default|GetSpearBox)))