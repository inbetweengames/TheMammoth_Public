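; Player controller for the Mammoth game that owns the main menu, HUD, options and credits widgets and shows subtitles with voice-over.
; At BeginPlay it creates the widgets, picking a touch or PC HUD by platform, then adds or removes them as the game flow state changes.
; A ForceTouch input swaps in the touch HUD.
; Subtitle requests are ignored while the ClearSubtitle timer runs, which also serves as the VO-playing check.
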(event Custom|SetSubtitle
  (params (text :type Text) (forDuration :type Float%20%28single-precision%29) (VO :type Sound%20Cue%20Object%20Reference))
  (if (not (Class|KismetSystemLibrary|IsTimerActive self "ClearSubtitle"))
    (Utilities|FlowControl|Sequence
      (:then_0
        (Class|MammothHudInterface|SetSubtitle(Message) (Variables|Default|GetHUD) text)
        (Utilities|Time|SetTimerbyFunctionName self "ClearSubtitle" forDuration))
      (:then_1
        (Audio|PlaySound2D self VO)))))

(event EventOnGameFlowStateChanged
  (params (newState :type EGameFlowState%20Enum :default "None"))
  (switch Utilities|FlowControl|Switch|SwitchonEGameFlowState newState
    (:MainMenu
      (UserInterface|Viewport|AddtoViewport (Variables|Default|GetMainMenu) 0))
    (:Intro
      (Widget|RemovefromParent (Variables|Default|GetMainMenu))
      (UserInterface|Viewport|AddtoViewport (Variables|Default|GetHUD) 0))
    (:InGame
      (UserInterface|Viewport|AddtoViewport (Variables|Default|GetHUD) 0)
      (Widget|RemovefromParent (Variables|Default|GetOptionsMenu)))
    (:Options
      (UserInterface|Viewport|AddtoViewport (Variables|Default|GetOptionsMenu) 0)
      (Widget|RemovefromParent (Variables|Default|GetHUD)))
    (:Credits
      (UserInterface|Viewport|AddtoViewport (Variables|Default|GetCreditsMenu) 0))))

(event EventBeginPlay
  (bind _self self)
  (bind _returnvalue (UserInterface|CreateWidget "/Game/Mammoth/UI/MainMenu_WB.MainMenu_WB_C" _self))
  (Variables|Default|SetMainMenu _returnvalue)
  (if (Class|TPTopDownPlayerController|IsMobilePlatform)
    (bind _returnvalue_2 (UserInterface|CreateWidget "/Game/Mammoth/UI/HUD_Touch_WB.HUD_Touch_WB_C"))
    (Variables|Default|SetHUD _returnvalue_2)
    (else
      (bind _returnvalue_3 (UserInterface|CreateWidget "/Game/Mammoth/UI/HUD_PC_WB.HUD_PC_WB_C" _self))
      (Variables|Default|SetHUD _returnvalue_3)))
  (bind _returnvalue_4 (UserInterface|CreateWidget "/Game/Mammoth/UI/OptionsMenu_WB.OptionsMenu_WB_C" self))
  (Variables|Default|SetOptionsMenu _returnvalue_4)
  (bind _returnvalue_5 (UserInterface|CreateWidget "/Game/Mammoth/UI/Credits_WB.Credits_WB_C" self))
  (Variables|Default|SetCreditsMenu _returnvalue_5))

(event Input|ActionEvents|InputActionForceTouch
  (params (Key :type Key%20Structure :default "AnyKey"))
  (:Pressed
    (if (Utilities|Enum|Equal(Enum) (Variables|Default|Getm_currentGameFlowState) "InGame")
      (Widget|RemovefromParent (Variables|Default|GetHUD))
      (bind _returnvalue (UserInterface|CreateWidget "/Game/Mammoth/UI/HUD_Touch_WB.HUD_Touch_WB_C" self))
      (bind _output_get (Variables|Default|SetHUD _returnvalue))
      (UserInterface|Viewport|AddtoViewport _output_get 0)
      (else
        (bind _returnvalue_2 (UserInterface|CreateWidget "/Game/Mammoth/UI/HUD_Touch_WB.HUD_Touch_WB_C" self))
        (Variables|Default|SetHUD _returnvalue_2)))))

(fn ConstructionScript)

(fn ClearSubtitle
  (Class|MammothHudInterface|SetSubtitle(Message) (Variables|Default|GetHUD)))

(fn IsVOPlaying
  (return (Class|KismetSystemLibrary|IsTimerActive self "ClearSubtitle")))